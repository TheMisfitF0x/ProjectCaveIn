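; BP_Car_2 is a car actor that travels along a spline on a referenced track, starting on BeginPlay when ActiveCar is set.
; A CarMovement timeline, with play rate set from Duration1 and start time from CarStartOffset, outputs an Alpha on each update.
; That Alpha is lerped across the spline's length to set the car's world location and rotation.
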(event `self.ReceiveBeginPlay`
  (if (`self.ActiveCar`)
    (`self.MoveCar_1`)))

(event `MoveCar_1`
  (bind _usefulspline (`/Game/DystopianCity_v1/BP_Car_Movement/BP_Track.UsefulSpline` (`self.TrackRef_1`)))
  (bind _returnvalue (`KismetMathLibrary.Lerp` 0.0 (`SplineComponent.GetSplineLength` _usefulspline) (`self.Alpha`)))
  (`TimelineComponent.SetPlayRate` (`self.CarMovement`) (/ 1.0 (`self.Duration_1`)))
  (`TimelineComponent.SetNewTime` (`self.CarMovement`) (`self.CarStartOffset`))
  (bind (_direction _alpha) (`Timeline|CarMovement`)
    (:`Update`
      (set `self.Alpha` _alpha)
      (`self.K2_SetActorLocationAndRotation` (`SplineComponent.GetLocationAtDistanceAlongSpline` _usefulspline _returnvalue "World") (`SplineComponent.GetRotationAtDistanceAlongSpline` _usefulspline _returnvalue "World")))))

(fn `UserConstructionScript`)
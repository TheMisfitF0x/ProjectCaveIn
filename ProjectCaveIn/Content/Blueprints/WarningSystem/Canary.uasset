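; Canary is a warning-system Blueprint that detects overlapping actors tagged Threat.
; Begin and end overlap events set and clear a single WarningActive flag, so any threat leaving clears the warning even if others remain.
; Tick prints the flag to screen and log every frame while it is true, as the only warning output.
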(event `self.ReceiveBeginPlay`)

(event `self.ReceiveActorBeginOverlap`
  (params (OtherActor :type "Actor Object Reference"))
  (if (`self.ActorHasTag` OtherActor "Threat")
    (set `self.WarningActive` true)))

(event `self.ReceiveActorEndOverlap`
  (params (OtherActor :type "Actor Object Reference"))
  (if (`self.ActorHasTag` OtherActor "Threat")
    (set `self.WarningActive` false)))

(event `self.ReceiveTick`
  (params (DeltaSeconds :type "Float (single-precision)"))
  (bind _warningactive (`self.WarningActive`))
  (`KismetSystemLibrary.PrintString` (`KismetStringLibrary.Conv_BoolToString` _warningactive) _warningactive _warningactive))

(fn `UserConstructionScript`)